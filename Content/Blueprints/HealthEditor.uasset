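; HealthEditor is an overlap trigger actor with a sprite that changes the HERO's health.
; Its configurable MySprite is applied to the PaperSprite component in both the construction script and BeginPlay.
; When the HERO overlaps its Box, it passes HealthAmount to ChangeHealth on that character, and it stays in the level afterward.
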(event OnComponentBeginOverlap(Box)
  (params (OverlappedComponent :type Primitive%20Component%20Object%20Reference) (OtherActor :type Actor%20Object%20Reference) (OtherComp :type Primitive%20Component%20Object%20Reference) (OtherBodyIndex :type Integer) (bFromSweep :type Boolean) (SweepResult :type Hit%20Result%20Structure%20%28by%20ref%29))
  (bind _ashero (Utilities|Casting|CastToHERO OtherActor))
  (Default|ChangeHealth _ashero (Variables|Default|GetHealthAmount)))

(event EventBeginPlay
  (Rendering|Components|Sprite|SetSprite (Variables|Default|GetPaperSprite) (Variables|Default|GetMySprite)))

(event Collision|EventActorBeginOverlap
  (params (OtherActor :type Actor%20Object%20Reference)))

(event EventTick
  (params (DeltaSeconds :type Float%20%28single-precision%29)))

(fn ConstructionScript
  (Rendering|Components|Sprite|SetSprite (Variables|Default|GetPaperSprite) (Variables|Default|GetMySprite)))