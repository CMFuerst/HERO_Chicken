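; HERO is a player-controlled 2D flipbook character with four-directional movement and animation.
; Two input axes drive movement along fixed world Y and negative X directions.
; Every tick, SetMyFlipbook updates the last move direction from input, prioritizing vertical over horizontal, and keeps it when input stops.
; Velocity then selects the Move or Idle flipbook for that direction, so the hero idles facing its last heading.
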(event EventTick
  (params (DeltaSeconds :type Float%20%28single-precision%29))
  (CallFunction|SetMyFlipbook))

(event Input|AxisEvents|InputAxisUpOrDown
  (params (AxisValue :type Float%20%28single-precision%29))
  (Pawn|Input|AddMovementInput "0,1.000000,0.000000" AxisValue false))

(event Input|AxisEvents|InputAxisLeftOrRight
  (params (AxisValue :type Float%20%28single-precision%29))
  (Pawn|Input|AddMovementInput "-1.000000,0.000000,0.000000" AxisValue false))

(fn ConstructionScript)

(fn SetMyFlipbook
  (if (or (!= (Input|AxisValues|GetLeftOrRight) 0.0) (!= (Input|AxisValues|GetUpOrDown) 0.0))
    (Variables|Default|SetLastMoveDirection (select (> (Input|AxisValues|GetUpOrDown) 0.0) "NewEnumerator0" (select (< (Input|AxisValues|GetUpOrDown) 0.0) "NewEnumerator1" (select (> (Input|AxisValues|GetLeftOrRight) 0.0) "NewEnumerator3" "NewEnumerator2")))))
  (Sprite|SetFlipbook (Variables|Default|GetSprite) (select (> (Math|Vector|VectorLength (Transformation|GetVelocity)) 0.0) (Utilities|Select :Index (Variables|Default|GetLastMoveDirection) :NewEnumerator0 "/Game/Character/Move_Up.Move_Up" :NewEnumerator1 "/Game/Character/Move_Down.Move_Down" :NewEnumerator2 "/Game/Character/Move_Left.Move_Left" :NewEnumerator3 "/Game/Character/Move_Right.Move_Right") (Utilities|Select :Index (Variables|Default|GetLastMoveDirection) :NewEnumerator0 "/Game/Character/Idle_Up.Idle_Up" :NewEnumerator1 "/Game/Character/Idle_Down.Idle_Down" :NewEnumerator2 "/Game/Character/Idle_Left.Idle_Left" :NewEnumerator3 "/Game/Character/Idle_Right.Idle_Right"))))